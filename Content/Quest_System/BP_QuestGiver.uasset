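; BP_QuestGiver is an interactable quest NPC or object that opens a quest giver screen for the player.
; Its trigger radius shows an interact prompt widget while the third-person character overlaps it, and Tick rotates that prompt to face the camera.
; Interact toggles a WB_QuestGiver viewport widget, switching the mouse cursor and input mode between Game-and-UI and game-only.
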(event OnComponentBeginOverlap(TriggerRadius)
  (params (OverlappedComponent :type Primitive%20Component%20Object%20Reference) (OtherActor :type Actor%20Object%20Reference) (OtherComp :type Primitive%20Component%20Object%20Reference) (OtherBodyIndex :type Integer) (bFromSweep :type Boolean) (SweepResult :type Hit%20Result%20Structure%20%28by%20ref%29))
  (Utilities|Casting|CastToBP_ThirdPersonCharacter OtherActor)
  (Rendering|SetVisibility (Variables|Default|GetInteract%20Widget) true false))

(event OnComponentEndOverlap(TriggerRadius)
  (params (OverlappedComponent :type Primitive%20Component%20Object%20Reference) (OtherActor :type Actor%20Object%20Reference) (OtherComp :type Primitive%20Component%20Object%20Reference) (OtherBodyIndex :type Integer))
  (Utilities|Casting|CastToBP_ThirdPersonCharacter OtherActor)
  (Rendering|SetVisibility (Variables|Default|GetInteract%20Widget) false false))

(event EventTick
  (params (DeltaSeconds :type Float%20%28single-precision%29))
  (Transformation|SetWorldRotation (Variables|Default|GetInteract%20Widget) (Math|Rotator|FindLookatRotation (Transformation|GetWorldLocation (Variables|Default|GetInteract%20Widget)) (Transformation|GetWorldLocation (Variables|/Script/Engine.PlayerCameraManager|GetTransformComponent (Game|GetPlayerCameraManager 0)))) false false))

(event EventInteract
  (bind _returnvalue (Game|GetPlayerController 0))
  (bind _returnvalue_2 (Game|GetPlayerController 0))
  (if (not (Variables|Default|GetWidget%20Active))
    (bind _returnvalue_3 (UserInterface|CreateWidget "/Game/Quest_System/WB_QuestGiver.WB_QuestGiver_C"))
    (bind _output_get (Variables|Default|SetQuest%20Widget _returnvalue_3))
    (UserInterface|Viewport|AddtoViewport _output_get 0)
    (Variables|Default|SetWidget%20Active true)
    (Variables|/Script/Engine.PlayerController|SetbShowMouseCursor _returnvalue_2 true)
    (Input|SetInputModeGameandUI _returnvalue_2 (Variables|Default|GetQuest%20Widget) "DoNotLock" true false)
    (else
      (Widget|RemovefromParent (Variables|Default|GetQuest%20Widget))
      (Variables|Default|SetQuest%20Widget 0)
      (Variables|Default|SetWidget%20Active false)
      (Variables|/Script/Engine.PlayerController|SetbShowMouseCursor _returnvalue false)
      (Input|SetInputModeGameOnly _returnvalue false))))

(fn ConstructionScript)