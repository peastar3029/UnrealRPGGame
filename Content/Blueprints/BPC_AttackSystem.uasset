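; BPC_AttackSystem is an attack component that handles sword attack input with a buffered combo.
; IA_Attack calls SwordAttack when CanAttack is true, which either saves the press during an attack or dispatches on AttackIndex.
; Only Attack1 is wired: a DoOnce-guarded, briefly delayed montage that advances the index.
; SwordAttackCombo consumes a saved press to dispatch again, otherwise StopCombo resets the state.
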(event Custom|Sword%20Attack
  ;[0.05127 0.05127 0.05127] Sword Attack
  (if (Variables|Default|Getis%20Attacking?)
    (Variables|Default|Setsave%20Attack? true)
    (else
      (Variables|Default|Setsave%20Attack? false)
      (switch int (Variables|Default|GetAttack%20Index)
        (:0
          (CallFunction|Attack1))))))

(event Custom|Sword%20Attack%20Combo
  ;[0.05127 0.05127 0.05127] Combo Continue
  (if (Variables|Default|Getsave%20Attack?)
    (Variables|Default|Setsave%20Attack? false)
    (switch int (Variables|Default|GetAttack%20Index)
      (:0
        (CallFunction|Attack1)))
    (else
      (CallFunction|StopCombo))))

(event Custom|Stop%20Combo
  ;[0.05127 0.05127 0.05127] Stop Combo / Attack
  (Variables|Default|Setis%20Attacking? false)
  (Variables|Default|SetAttack%20Index 0))

(event Custom|Attack1
  ;[0.05127 0.05127 0.05127] Attack1
  (Utilities|FlowControl|DoOnce false :!label _label
    (:Completed
      (Utilities|FlowControl|Delay 0.1)
      (Animation|Montage|PlayMontage 0 0
        (:then
          (Variables|Default|SetAttack%20Index 1)
          (goto _label Reset))))))

(event Input|EnhancedActionEvents|EnhancedInputActionIA_Attack
  (params (ActionValue :type Boolean) (ElapsedSeconds :type Float%20%28double-precision%29) (TriggeredSeconds :type Float%20%28double-precision%29) (InputAction :type Input%20Action%20Object%20Reference :default "/Game/ThirdPerson/Input/Actions/IA_Attack.IA_Attack"))
  ;[0.05127 0.05127 0.05127] Attack Input
  (:Started
    (if (Variables|Default|Getcan%20Attack?)
      (CallFunction|SwordAttack))))